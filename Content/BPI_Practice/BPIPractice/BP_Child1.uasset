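; BP_Child1 is a child pickup actor in a Blueprint Interface practice project that sends a "Green!" item name and text color to whatever overlaps it.
; Its Sphere overlap event calls the BPI PickUpItem message on the other actor, which takes effect only if that actor implements the interface.
; An older cast to BP_ThirdPersonCharacter with a direct PickUpItem call remains unconnected.
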(event `self.Sphere.OnComponentBeginOverlap`
  (params (OverlappedComponent :type "PrimitiveComponent Object Reference") (OtherActor :type "Actor Object Reference") (OtherComp :type "PrimitiveComponent Object Reference") (OtherBodyIndex :type Integer) (bFromSweep :type Boolean) (SweepResult :type "HitResult Structure (by ref)"))
  ; そのアクターがBPIで作成した関数を実装していたらその関数を実行
  (message `/Game/BPI_Practice/BPIPractice/BPI_PickUpItem.BPIPickUpItem` OtherActor "Green!" (struct :`R` 1.0 :`B` 0.61752 :`A` 1.0)))

(fn `UserConstructionScript`
  (`parent.UserConstructionScript`))